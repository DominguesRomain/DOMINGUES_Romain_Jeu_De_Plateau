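; BP_NavDestination is an actor that periodically jumps to a random position, apparently serving as a roaming AI navigation target.
; From BeginPlay it loops forever, waiting on a fixed Delay before each SetActorLocation.
; X and Y each average two scaled random floats, biasing toward mid-range, then clamp to set bounds while Z stays unchanged.
; The X clamp piles many results on its lower bound, while the Y range never reaches its clamp.
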(event `self.ReceiveBeginPlay`
  (bind (_returnvalue_x _returnvalue_y _returnvalue_z) (`KismetMathLibrary.BreakVector` (`self.K2_GetActorLocation`)))
  (`KismetSystemLibrary.Delay` 9.0 :!label _label)
  (`self.K2_SetActorLocation` (`KismetMathLibrary.MakeVector` (`KismetMathLibrary.FClamp` (/ (+ (* (`KismetMathLibrary.RandomFloat`) 26000.0) (* (`KismetMathLibrary.RandomFloat`) 26000.0)) 2.0) 11500.0 23550.0) (`KismetMathLibrary.FClamp` (/ (+ (* (`KismetMathLibrary.RandomFloat`) -8500.0) (* (`KismetMathLibrary.RandomFloat`) 8500.0)) 2.0) -6283.0 4651.0) _returnvalue_z))
  (goto _label))

(fn `UserConstructionScript`)