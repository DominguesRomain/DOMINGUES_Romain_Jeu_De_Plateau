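; BP_SpawnPiece spawns BP_Piece collectibles in one of five lanes during a minigame.
; On BeginPlay it registers itself with the inst GameInstance; startminigame then loops while InMinigame is set, waiting random delays that shorten when Time drops below 31.
; Spawnpiece chooses the lane's Y through nested random checks at fixed X and Z, re-rolling at each check, so lanes are not equally likely.
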(event `self.ReceiveBeginPlay`
  (bind _asinst (cast `/Game/bluprint/systeme/inst` (`GameplayStatics.GetGameInstance`)))
  (bind _output_get (set `self.As Inst` _asinst))
  (set `/Game/bluprint/systeme/inst.spawnerpiece` self _output_get))

(event `startminigame`
  (while (`/Game/bluprint/systeme/inst.in minigame` (`self.As Inst`)) :!label _label
    (if (< (`/Game/bluprint/systeme/inst.Time` (`self.As Inst`)) 31)
      (`KismetSystemLibrary.Delay` (+ (* (`KismetMathLibrary.RandomFloat`) 0.65) 0.3))
      (else
        (`KismetSystemLibrary.Delay` (+ (* (`KismetMathLibrary.RandomFloat`) 1.6) 0.8))))
    (`self.Spawnpiece`)
    (goto _label)))

(fn `Spawnpiece`
  (bind _returnvalue (`KismetMathLibrary.RandomIntegerInRange` 1 5))
  ;[1 0.1346 0] choix du couloir
  (if (<= _returnvalue 1)
    (set `self.ValueY` -8500.0)
    (`|SpawnActorFromClass` "/Game/bluprint/CollecteBP/BP_Piece.BP_Piece_C" (`KismetMathLibrary.MakeTransform` (`KismetMathLibrary.MakeVector` 30800.0 (`self.ValueY`) 600.0) (struct) (3.0 3.0 3.0)) "AlwaysSpawn" "MultiplyWithRoot" null null :!label _label)
    (elif (<= _returnvalue 2)
      (set `self.ValueY` -5000.0)
      (goto _label)
      (elif (<= _returnvalue 3)
        (set `self.ValueY` -1500.0)
        (goto _label)
        (elif (<= _returnvalue 4)
          (set `self.ValueY` 2000.0)
          (goto _label)
          (elif (<= _returnvalue 6)
            (set `self.ValueY` 5500.0)
            (goto _label)
            (else
              (`KismetSystemLibrary.PrintString` "erreur list"))))))))

(fn `UserConstructionScript`)