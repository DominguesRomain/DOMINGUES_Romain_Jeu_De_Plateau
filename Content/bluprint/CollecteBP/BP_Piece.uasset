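; BP_Piece is a minigame coin that moves along negative X and spins, driven by a timeline.
; On BeginPlay, SuperValue is boosted when game-instance Time is low, and randomly for super coins, which also change material.
; SuperValue scales movement and rotation, and its thresholds pick score amounts.
; Overlapping the player's PionCollecte adds score, while reaching the game instance's Spawnerpiece subtracts it; both destroy the coin.
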(event `self.ReceiveBeginPlay`
  (bind (_returnvalue_x _returnvalue_y _returnvalue_z) (`KismetMathLibrary.BreakVector` (`self.K2_GetActorLocation`)))
  (bind _asbp_player (cast `/Game/bluprint/systeme/BP_Player` (`GameplayStatics.GetPlayerPawn` 0)))
  (set `self.As BP Player` _asbp_player)
  (bind _asinst (cast `/Game/bluprint/systeme/inst` (`GameplayStatics.GetGameInstance`)))
  (set `self.As Inst` _asinst)
  ;[1 0 0.05096] super coin
  (if (not (> (`/Game/bluprint/systeme/inst.Time` (`self.As Inst`)) 29))
    (set `self.SuperValue` (* (`self.SuperValue`) 1.8)))
  (if (<= (`KismetMathLibrary.RandomIntegerInRange` 1 5) 1)
    (set `self.SuperValue` (+ (`self.SuperValue`) 1.9))
    (`PrimitiveComponent.CreateDynamicMaterialInstance` (`self.piece`) 0 "/Game/bluprint/CollecteBP/pie/M_Piece_Inst1.M_Piece_Inst1" "None")
    (bind (_direction _newtrack_0) (`Timeline|Chronologie` :!label _label)
      (:`Update`
        (`self.K2_SetActorLocationAndRotation` (`KismetMathLibrary.MakeVector` (- _returnvalue_x (* _newtrack_0 (* (`self.SuperValue`) 1.8))) _returnvalue_y _returnvalue_z) (`KismetMathLibrary.MakeRotator` 0.0 0.0 (* _newtrack_0 (* (`self.SuperValue`) 2.6))))))
    (else
      (goto _label))))

(event `self.Sphere.OnComponentBeginOverlap`
  (params (OverlappedComponent :type "PrimitiveComponent Object Reference") (OtherActor :type "Actor Object Reference") (OtherComp :type "PrimitiveComponent Object Reference") (OtherBodyIndex :type Integer) (bFromSweep :type Boolean) (SweepResult :type "HitResult Structure (by ref)"))
  (bind _as_inst (`self.As Inst`))
  (bind _as_inst_2 (`self.As Inst`))
  (bind _scoreminijeu (`/Game/bluprint/systeme/inst.ScoreMiniJeu` _as_inst))
  (bind _scoreminijeu_2 (`/Game/bluprint/systeme/inst.ScoreMiniJeu` _as_inst_2))
  ;[1 1 1] ki deteck ai komte lé pauin
  (if (== (`/Game/bluprint/systeme/BP_Player.PionCollecte` (`self.As BP Player`)) OtherActor)
    (if (> (`self.SuperValue`) 2.4)
      (set `/Game/bluprint/systeme/inst.ScoreMiniJeu` (+ _scoreminijeu 3.0) _as_inst)
      (else
        (`/Engine/EditorBlueprintResources/StandardMacros.IncrementFloat` _scoreminijeu
          (:`  `
            _))))
    (`self.K2_DestroyActor`)
    (elif (== OtherActor (`/Game/bluprint/systeme/inst.spawnerpiece` _as_inst_2))
      (if (> (`self.SuperValue`) 2.0)
        (set `/Game/bluprint/systeme/inst.ScoreMiniJeu` (- _scoreminijeu_2 1.5) _as_inst_2)
        (else
          (set `/Game/bluprint/systeme/inst.ScoreMiniJeu` (- _scoreminijeu_2 0.5) _as_inst_2)))
      (`self.K2_DestroyActor`))))

(fn `UserConstructionScript`)