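; BP_Pion1 is a player pawn piece that moves between cells in a turn-based game.
; MoveToNewCell places it at the cell position, offset by the GameMode's PlayerTurn, and copies that player's score from the GameInstance list.
; While Vroum is set, Tick plays a Timeline that shifts it along X through a sine.
; ColorVroum applies a random material to Arrete and removes it from the supplied list.
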(event `self.ReceiveBeginPlay`
  (bind _asgm (cast `/Game/bluprint/systeme/GM` (`GameplayStatics.GetGameMode`)))
  (set `self.As GM` _asgm)
  (bind _asinst (cast `/Game/bluprint/systeme/inst` (`GameplayStatics.GetGameInstance`)))
  (set `self.As Inst` _asinst))

(event `MoveToNewCell`
  (params (NewCellPosition :type "Vector Structure"))
  (bind _playerturn (`/Game/bluprint/systeme/GM.PlayerTurn` (`self.As GM`)))
  (bind (_output_playerid _output_score) (break `/Game/bluprint/systeme/struc` (`|GetArrayItem` (`/Game/bluprint/systeme/inst.plist` (`self.As Inst`)) _playerturn)))
  (`self.K2_SetActorLocation` (`KismetMathLibrary.MakeVector` (- (+ NewCellPosition_X (* _playerturn 140)) 350.0) (- (+ NewCellPosition_Y (* _playerturn 10)) 5.0)))
  (set `self.ListInfoScore` _output_score))

(event `self.ReceiveTick`
  (params (DeltaSeconds :type "Float (single-precision)"))
  (bind (_returnvalue_x _returnvalue_y _returnvalue_z) (`KismetMathLibrary.BreakVector` (`self.K2_GetActorLocation`)))
  (if (`self.Vroum`)
    (bind (_direction _newtrack_0) (`Timeline|Timeline`)
      (:`Update`
        (`self.K2_SetActorLocation` (`KismetMathLibrary.MakeVector` (+ (* (`KismetMathLibrary.Sin` _newtrack_0) 8.0) _returnvalue_x) _returnvalue_y _returnvalue_z))))))

(fn `ColorVroum`
  (params (ListMat :type "Array of Material Object Reference"))
  (bind _newparam (`self.randomColr` ListMat))
  (`KismetArrayLibrary.Array_RemoveItem` ListMat _newparam)
  (`PrimitiveComponent.CreateDynamicMaterialInstance` (`self.Arrete`) 0 _newparam "None"))

(fn `randomColr`
  (params (NewParam1 :type "Array of Material Object Reference"))
  (returns (NewParam :type "Material Object Reference"))
  (return (`KismetArrayLibrary.Array_Random` NewParam1)))

(fn `UserConstructionScript`)