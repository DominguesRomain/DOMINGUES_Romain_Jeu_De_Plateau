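; BP_Board is the game board actor, holding a list of cells that other code queries by index.
; On BeginPlay it registers itself as Board on the GM game mode and stores the last cell index as NbCell.
; Lookup functions return a cell's world location, only for indices below NbCell, or its CaseType, which is also printed and not bounds-checked.
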(event `self.ReceiveBeginPlay`
  (bind _asgm (cast `/Game/bluprint/systeme/GM` (`GameplayStatics.GetGameMode`)))
  (bind _output_get (set `self.As GM` _asgm))
  (set `/Game/bluprint/systeme/GM.Board` self _output_get)
  (set `self.NbCell` (- (`KismetArrayLibrary.Array_Length` (`self.CellList`)) 1)))

(fn `GetCellPositionByNumber`
  (params (CellIndex :type Integer))
  (returns (CellLocation :type "Vector Structure"))
  (if (< CellIndex (`self.NbCell`))
    (return (`self.K2_GetActorLocation` (`|GetArrayItem` (`self.CellList`) CellIndex)))))

(fn `GetCellTypeByName`
  (params (CellIndex :type Integer))
  (returns (CellType :type Name))
  (bind _casetype (`/Game/bluprint/Cube/BP_Cell.CaseType` (`|GetArrayItem` (`self.CellList`) CellIndex)))
  (`KismetSystemLibrary.PrintString` (`KismetStringLibrary.Conv_NameToString` _casetype) true true (struct :`G` 0.66 :`B` 1.0 :`A` 1.0) 6.0)
  (return _casetype))

(fn `UserConstructionScript`)