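; BP_Pion is a game piece ("pion") that moves between cells, apparently on a turn-based board.
; On BeginPlay it casts the game mode to GM and stores the reference.
; Its MoveToNewCell event teleports it to the given cell position at a fixed height, with X and Y offsets scaled by the GM's current PlayerTurn so each player's piece lands at a different spot.
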(event `self.ReceiveBeginPlay`
  (bind _asgm (cast `/Game/bluprint/systeme/GM` (`GameplayStatics.GetGameMode`)))
  (set `self.As GM` _asgm))

(event `MoveToNewCell`
  (params (NewCellPosition :type "Vector Structure"))
  (bind _playerturn (`/Game/bluprint/systeme/GM.PlayerTurn` (`self.As GM`)))
  (`self.K2_SetActorLocation` (`KismetMathLibrary.MakeVector` (- (+ NewCellPosition_X (* _playerturn 20)) 60.0) (- (+ NewCellPosition_Y (* _playerturn 60)) 100.0) 60.0)))

(fn `UserConstructionScript`)