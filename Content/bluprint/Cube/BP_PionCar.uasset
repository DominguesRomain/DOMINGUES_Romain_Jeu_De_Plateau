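; Car player pawn for a board game that AI-moves to cells with a per-turn offset, then reads the current player's score from the game instance.
; While Vroum is set, Tick plays a timeline whose sine output jitters the car along X.
; ColorVroum reuses the material stored in the game instance or draws an unused random one.
; Left/right collect functions shift the car between bounded lanes relative to a given pawn.
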(event `self.ReceiveBeginPlay`
  ;[0.5171 1 0.8689] Vroum Vroum les voitures
  (bind _asgm (cast `/Game/bluprint/systeme/GM` (`GameplayStatics.GetGameMode`)))
  (set `self.As GM` _asgm)
  (bind _asinst (cast `/Game/bluprint/systeme/inst` (`GameplayStatics.GetGameInstance`)))
  (set `self.As Inst` _asinst))

(event `MoveToNewCell`
  (params (NewParam :type "Vector Structure"))
  (bind _playerturn (`/Game/bluprint/systeme/GM.PlayerTurn` (`self.As GM`)))
  (bind (_output_playerid _output_score) (break `/Game/bluprint/systeme/struc` (`|GetArrayItem` (`/Game/bluprint/systeme/inst.plist` (`self.As Inst`)) _playerturn)))
  ;[0.5171 1 0.8689] Vroum Vroum les voitures
  (`SceneComponent.K2_SetWorldRotation` (`self.Car`) (struct :`Yaw` 90.0) false false)
  (`|AIMoveTo` self (`KismetMathLibrary.MakeVector` (- (+ NewParam_X (* _playerturn 175)) 460.0) (- (+ NewParam_Y (* _playerturn 10)) 50.0)) null
    (:`then`
      (set `self.ListInfoScore` _output_score))))

(event `self.ReceiveTick`
  (params (DeltaSeconds :type "Float (single-precision)"))
  (bind (_returnvalue_x _returnvalue_y _returnvalue_z) (`KismetMathLibrary.BreakVector` (`self.K2_GetActorLocation`)))
  ;[1 0.4925 0.1331] mouvement perpetuelle de la voiture
  (if (`self.Vroum`)
    (bind (_direction _newtrack_0) (`Timeline|Timeline`)
      (:`Update`
        (`self.K2_SetActorLocation` (`KismetMathLibrary.MakeVector` (+ (* (`KismetMathLibrary.Sin` _newtrack_0) 8.0) _returnvalue_x) _returnvalue_y _returnvalue_z))))))

(fn `ColorVroum`
  (params (ListMat :type "Array of Material Object Reference") (PawnNB :type Integer))
  (returns (Mat :type "Material Object Reference"))
  (bind (_value _returnvalue) (`BlueprintMapLibrary.Map_Find` (`/Game/bluprint/systeme/inst.ListColor` (`self.As Inst`)) PawnNB))
  ;[1 0.2483 0] Attribution d'une couleur, et mémoire de la couleur pour la partie
  (if _returnvalue
    (set `self.DejaPimp` true)
    (`PrimitiveComponent.CreateDynamicMaterialInstance` (`self.Arrete`) 0 _value "None")
    (return _value)
    (else
      (bind _newparam (`self.randomColr` ListMat))
      (`KismetArrayLibrary.Array_RemoveItem` ListMat _newparam)
      (`PrimitiveComponent.CreateDynamicMaterialInstance` (`self.Arrete`) 0 _newparam "None")
      (return _newparam))))

(fn `MoveLeftCollect`
  (params (PionCollect :type "/Game/bluprint/Cube/BP_PionCar Object Reference"))
  (bind (_returnvalue_x _returnvalue_y _returnvalue_z) (`KismetMathLibrary.BreakVector` (`self.K2_GetActorLocation` PionCollect)))
  (set `self.PionCollecte` PionCollect)
  (if (not (< (`self.PlacementCollecte`) -1))
    (`/Engine/EditorBlueprintResources/StandardMacros.DecrementInt` (`self.PlacementCollecte`)
      (:`  `
        (`self.K2_SetActorLocation` (`KismetMathLibrary.MakeVector` _returnvalue_x (- _returnvalue_y 3500.0) _returnvalue_z))))))

(fn `MoveRightCollect`
  (params (PionCollect :type "/Game/bluprint/Cube/BP_PionCar Object Reference"))
  (bind (_returnvalue_x _returnvalue_y _returnvalue_z) (`KismetMathLibrary.BreakVector` (`self.K2_GetActorLocation` PionCollect)))
  (set `self.PionCollecte` PionCollect)
  (if (not (> (`self.PlacementCollecte`) 1))
    (`/Engine/EditorBlueprintResources/StandardMacros.IncrementInt` (`self.PlacementCollecte`)
      (:`  `
        (`self.K2_SetActorLocation` (`KismetMathLibrary.MakeVector` _returnvalue_x (+ _returnvalue_y 3500.0) _returnvalue_z))))))

(fn `randomColr`
  (params (NewParam1 :type "Array of Material Object Reference"))
  (returns (NewParam :type "Material Object Reference"))
  (return (`KismetArrayLibrary.Array_Random` NewParam1)))

(fn `UserConstructionScript`)