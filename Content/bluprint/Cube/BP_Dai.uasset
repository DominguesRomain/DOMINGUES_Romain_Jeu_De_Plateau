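; BP_Dai is a physics-driven die that is thrown and reports the face it lands on.
; CastDice resets the die with random rotation, applies randomized linear and radial impulses, then waits a fixed delay before calling RollDai.
; RollDai maps the first component overlapping BoxJudge to one of six box values, subtracts it from DaiType + 1 for the opposite face, and prints the result.
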(event `self.ReceiveBeginPlay`
  (`SceneComponent.K2_SetRelativeLocation` (`self.BoxJudge`) (9379.930376 18380.886503 -779.810136) false true))

(event `CastDice`
  (bind _returnvalue (`KismetMathLibrary.RandomFloat`))
  (bind _dai (`self.dai`))
  (bind _dai_2 (`self.dai`))
  (bind (_returnvalue_x _returnvalue_y _returnvalue_z) (`KismetMathLibrary.BreakVector` (`SceneComponent.K2_GetComponentLocation` _dai_2)))
  (bind _returnvalue_2 (* (`KismetMathLibrary.RandomFloat`) 180.0))
  (bind _returnvalue_3 (+ (* _returnvalue 30.0) 2.0))
  (`SceneComponent.K2_SetRelativeTransform` _dai_2 (`KismetMathLibrary.MakeTransform` (2390.0 -1050.0 4500.0) (`KismetMathLibrary.MakeRotator` _returnvalue_2 _returnvalue_2 _returnvalue_2) (1000.0 1000.0 1000.0)) false true)
  (set `self.Map` (`|MakeMap` (`self.Box1`) 1 (`self.Box2`) 2 (`self.Box3`) 3 (`self.Box4`) 4 (`self.Box5`) 5 (`self.Box6`) 6 :!type "ActorComponent Object Reference"))
  (`KismetSystemLibrary.Delay` 0.2)
  (`PrimitiveComponent.AddImpulse` _dai (`KismetMathLibrary.MakeVector` (* _returnvalue_3 2500.0) (* _returnvalue_3 300.0) -150000.0) "None" false)
  (`PrimitiveComponent.AddRadialImpulse` _dai (`KismetMathLibrary.MakeVector` (* _returnvalue_x 10.0) _returnvalue_y (* _returnvalue_z -4.0)) (+ (* _returnvalue 900.0) 1500.0) (* (+ (* _returnvalue 10.0) 20.0) 1200000.0) "RIF_Constant" false)
  (`KismetSystemLibrary.Delay` 6.5)
  (`self.Roll Dai`))

(fn `Roll Dai`
  (set `self.stableValue` true)
  (set `self.DaiResult` 0)
  (for _ (range (+ (`self.DaiNumber`) 1))
    _)
  (bind _output_get (set `self.DaiResult` (+ (`self.DaiResult`) (- (+ (`self.DaiType`) 1) (`BlueprintMapLibrary.Map_Find` (`self.Map`) (`|GetArrayItem` (`PrimitiveComponent.GetOverlappingComponents` (`self.BoxJudge`))))))))
  (`KismetSystemLibrary.PrintString` (`KismetStringLibrary.Conv_IntToString` _output_get) true true (struct :`R` 1.0 :`B` 0.39707 :`A` 1.0)))

(fn `UserConstructionScript`)