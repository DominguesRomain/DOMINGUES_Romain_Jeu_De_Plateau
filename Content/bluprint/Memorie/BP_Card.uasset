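; BP_Card is a clickable, two-sided card actor, apparently for a memory game, whose Color enum sets the Verso material in the construction script.
; A click, unless blocked by the Anticlique flag reached through the GM game mode, flips the card and after a short delay passes it to GM's QuandCarteClique.
; TournerLesCartes toggles Isclickable and snaps the root rotation between two sides based on its current roll.
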(event `self.ReceiveBeginPlay`
  (bind _asgm (cast `/Game/bluprint/systeme/GM` (`GameplayStatics.GetGameMode`)))
  (set `self.As GM` _asgm))

(event `self.ReceiveActorOnClicked`
  (params (ButtonPressed :type "Key Structure"))
  (if (`/Game/bluprint/systeme/inst.anticlique` (`/Game/bluprint/systeme/GM.As Inst` (`self.As GM`)))
    _
    (elif (`self.isclickable`)
      (`self.TournerLesCartes`)
      (`KismetSystemLibrary.Delay` 0.5)
      (`/Game/bluprint/systeme/GM.QuandCarteClique` (`self.As GM`) self))))

(fn `ChangeColor`
  (switch `/Game/bluprint/Memorie/énummemo` (`self.Color`)
    (:`NewEnumerator0`
      (`PrimitiveComponent.SetMaterial` (`self.Verso`) 0 "/Game/bluprint/ElementLD/asset/voiture/UltraVioletIndice50.UltraVioletIndice50"))
    (:`NewEnumerator1`
      (`PrimitiveComponent.SetMaterial` (`self.Verso`) 0 "/Game/bluprint/ElementLD/asset/voiture/JauneDeRyanGooseling.JauneDeRyanGooseling"))
    (:`NewEnumerator2`
      (`PrimitiveComponent.SetMaterial` (`self.Verso`) 0 "/Game/bluprint/ElementLD/asset/voiture/TurquoiseSupra-Néon.TurquoiseSupra-Néon"))
    (:`NewEnumerator3`
      (`PrimitiveComponent.SetMaterial` (`self.Verso`) 0 "/Game/bluprint/ElementLD/asset/voiture/RougeDémonDeLaPiste.RougeDémonDeLaPiste"))))

(fn `TournerLesCartes`
  (bind _returnvalue_roll (`KismetMathLibrary.BreakRotator` (`SceneComponent.K2_GetComponentRotation` (`self.DefaultSceneRoot`))))
  (set `self.isclickable` (not (`self.isclickable`)))
  (if (== _returnvalue_roll 0.0)
    (`SceneComponent.K2_SetRelativeRotation` (`self.DefaultSceneRoot`) (`KismetMathLibrary.MakeRotator` 180.0 90.0 180.0) false false)
    (else
      (`SceneComponent.K2_SetRelativeRotation` (`self.DefaultSceneRoot`) (`KismetMathLibrary.MakeRotator` 0.0 90.0 180.0) false false))))

(fn `UserConstructionScript`
  (`self.ChangeColor`))