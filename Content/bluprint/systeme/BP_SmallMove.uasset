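; BP_SmallMove is an actor that shifts itself vertically by small amounts, upward or downward depending on the Up flag.
; Each Tick plays one of two timelines, Timeline or Chronologie, based on that flag, which this graph never changes.
; Their updates add a scaled sine of the track value to the current Z, so the offset accumulates while X and Y stay unchanged.
; A separate Move function increments a float but is never called here.
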(event `self.ReceiveTick`
  (params (DeltaSeconds :type "Float (single-precision)"))
  (bind (_returnvalue_x _returnvalue_y _returnvalue_z) (`KismetMathLibrary.BreakVector` (`self.K2_GetActorLocation`)))
  (bind (_returnvalue_x_2 _returnvalue_y_2 _returnvalue_z_2) (`KismetMathLibrary.BreakVector` (`self.K2_GetActorLocation`)))
  (if (`self.Up`)
    (bind (_direction _newtrack_0) (`Timeline|Timeline` :`NewTime` 100000.0)
      (:`Update`
        (`AddComponent|NODE_AddUniformVector-0`)
        (`self.K2_SetActorLocation` (`KismetMathLibrary.MakeVector` _returnvalue_x_2 _returnvalue_y_2 (+ (* (`KismetMathLibrary.Sin` _newtrack_0) 1.2) _returnvalue_z_2)))))
    (else
      (bind (_direction_2 _newtrack_0_2) (`Timeline|Chronologie` :`NewTime` 100000.0)
        (:`Update`
          (`AddComponent|NODE_AddUniformVector-1`)
          (`self.K2_SetActorLocation` (`KismetMathLibrary.MakeVector` _returnvalue_x _returnvalue_y (+ _returnvalue_z (* (`KismetMathLibrary.Sin` _newtrack_0_2) -1.2)))))))))

(fn `Move`
  (params (Float :type "Float (double-precision)"))
  (`/Engine/EditorBlueprintResources/StandardMacros.IncrementFloat` Float))

(fn `UserConstructionScript`)