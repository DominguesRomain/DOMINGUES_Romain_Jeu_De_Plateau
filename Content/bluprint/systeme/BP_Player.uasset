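; Player input Blueprint for a dice board game, driving turns through the GM game mode and turn counters in the game instance.
; G plays a timed turn (define player, roll, move, case effect, save), with AutoIA blocking re-entry.
; With AutoActivate, a latent Loop macro chains further turns until PlayerTurn reaches NbOfPlayer.
; P adds a player, J calls the game mode's Juke, and B opens the main menu level.
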(event `self.ReceiveBeginPlay`
  (bind _asgm (cast `/Game/bluprint/systeme/GM` (`GameplayStatics.GetGameMode`)))
  (set `self.As GM` _asgm)
  (bind _asinst (cast `/Game/bluprint/systeme/inst` (`GameplayStatics.GetGameInstance`)))
  (set `self.As Inst` _asinst))

(event `Key|G`
  (params (Key :type "Key Structure"))
  (bind _as_gm (`self.As GM`))
  (bind _as_gm_2 (`self.As GM`))
  (bind _as_inst (`self.As Inst`))
  ;[0.2024 1 0] Lance Un tour de jeu (Dé + move pawn)
  (:`Pressed`
    (if (`/Game/bluprint/systeme/GM.Start` _as_gm)
      (if (`self.AutoIA`)
        (set `self.AutoIA` false)
        (`/Game/bluprint/systeme/inst.GlobalTurnCount` _as_inst)
        (`/Game/bluprint/systeme/inst.TotalTurnCount` _as_inst)
        (`/Game/bluprint/systeme/GM.DefinePlayer` _as_gm)
        (`/Game/bluprint/systeme/GM.Lance le dai` _as_gm)
        (`KismetSystemLibrary.Delay` 7.0)
        (`/Game/bluprint/systeme/GM.RollADaiAndMove` _as_gm)
        (`KismetSystemLibrary.Delay` 3.5)
        (`/Game/bluprint/systeme/GM.CaseEffectApply` _as_gm)
        (`/Game/bluprint/systeme/GM.SaveAllValue` _as_gm)
        (`KismetSystemLibrary.Delay` 1.5)
        (set `self.AutoIA` true)
        (if (`self.AutoActivate`)
          ;[1 1 1] Mode Auto
          (set `self.AutoIA` false)
          (`self.Loop` (!= (`/Game/bluprint/systeme/GM.PlayerTurn` _as_gm_2) (`/Game/bluprint/systeme/GM.NbOfPlayer` _as_gm_2)) 0.5 :!label _label
            (:`NewParam3`
              (`KismetSystemLibrary.Delay` 2.0)
              (`/Game/bluprint/systeme/inst.TotalTurnCount` (`self.As Inst`))
              (`/Game/bluprint/systeme/GM.DefinePlayer` _as_gm_2)
              (`/Game/bluprint/systeme/GM.Lance le dai` _as_gm_2)
              (`KismetSystemLibrary.Delay` 7.0)
              (`/Game/bluprint/systeme/GM.RollADaiAndMove` _as_gm_2)
              (`KismetSystemLibrary.Delay` 3.5)
              (`/Game/bluprint/systeme/GM.CaseEffectApply` _as_gm_2)
              (`/Game/bluprint/systeme/GM.SaveAllValue` _as_gm_2)
              (`KismetSystemLibrary.Delay` 1.5)
              (goto _label))
            (:`NewParam4`
              (set `self.AutoIA` true))))))))

(event `Key|J`
  (params (Key :type "Key Structure"))
  (:`Pressed`
    (`/Game/bluprint/systeme/GM.Juke` (`self.As GM`))))

(event `Key|P`
  (params (Key :type "Key Structure"))
  ;[1 0 0.1891] Ajoute un joueur
  (:`Pressed`
    (`/Game/bluprint/systeme/GM.AddPlayer` (`self.As GM`))))

(event `Key|B`
  (params (Key :type "Key Structure"))
  (:`Pressed`
    (`GameplayStatics.OpenLevelBySoftObjectPtr` "/Game/map/OpenMainMenu.OpenMainMenu")))

(fn `UserConstructionScript`)