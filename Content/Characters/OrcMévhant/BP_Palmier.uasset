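; Palm tree actor that spawns coconut fruit (BP_Fruit) around itself using two timed random-chance loops started at BeginPlay.
; One loop spawns elevated fruit into a list until a counter reaches three; the other endlessly scatters untracked fruit farther out at the actor's height.
; PerteFruit enables physics on the oldest listed fruit and delists it, without lowering the counter.
; Capsule overlap stores any overlapping AIC_NPC reference.
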(event `2e part`
  (bind (_returnvalue_x _returnvalue_y _returnvalue_z) (`KismetMathLibrary.BreakVector` (`self.K2_GetActorLocation`)))
  (`KismetSystemLibrary.Delay` 3.5 :!label _label)
  (if (<= (`KismetMathLibrary.RandomFloat`) 0.31)
    (`|SpawnActorFromClass` "/Game/bluprint/Cube/BP_Fruit.BP_Fruit_C" (`KismetMathLibrary.MakeTransform` (`KismetMathLibrary.MakeVector` (+ (`KismetMathLibrary.RandomFloatInRange` 2000.0 -2000.0) _returnvalue_x) (+ _returnvalue_y (`KismetMathLibrary.RandomFloatInRange` 2000.0 -2000.0)) _returnvalue_z) (struct) (6.0 6.0 6.0)) "AdjustIfPossibleButAlwaysSpawn" "MultiplyWithRoot" null null)
    (goto _label)
    (else
      (goto _label))))

(event `self.ReceiveBeginPlay`
  (bind (_returnvalue_x _returnvalue_y _returnvalue_z) (`KismetMathLibrary.BreakVector` (`self.K2_GetActorLocation`)))
  (`self.2e part`)
  (if (< (`self.Fruit`) 3) :!label _label_2
    (`KismetSystemLibrary.Delay` 7.0)
    (if (<= (`KismetMathLibrary.RandomFloat`) 0.5)
      (bind _returnvalue (`|SpawnActorFromClass` "/Game/bluprint/Cube/BP_Fruit.BP_Fruit_C" (`KismetMathLibrary.MakeTransform` (`KismetMathLibrary.MakeVector` (+ (`KismetMathLibrary.RandomFloatInRange` 800.0 -800.0) _returnvalue_x) (+ _returnvalue_y (`KismetMathLibrary.RandomFloatInRange` 800.0 -800.0)) (+ _returnvalue_z 1800.0)) (struct) (6.0 6.0 6.0)) "AdjustIfPossibleButAlwaysSpawn" "MultiplyWithRoot" null null))
      (`KismetArrayLibrary.Array_Add` (`self.ListeFruit`) _returnvalue)
      (`/Engine/EditorBlueprintResources/StandardMacros.IncrementInt` (`self.Fruit`)
        (:`  `
          (goto _label_2)))
      (else
        (goto _label_2)))))

(event `self.Capsule.OnComponentBeginOverlap`
  (params (OverlappedComponent :type "PrimitiveComponent Object Reference") (OtherActor :type "Actor Object Reference") (OtherComp :type "PrimitiveComponent Object Reference") (OtherBodyIndex :type Integer) (bFromSweep :type Boolean) (SweepResult :type "HitResult Structure (by ref)"))
  (bind _asaic_npc (cast `/Game/Characters/OrcMévhant/AIC_NPC` OtherActor))
  (set `self.As AIC NPC` _asaic_npc))

(fn `Perte fruit`
  (bind _listefruit (`self.ListeFruit`))
  (bind _output (`|GetArrayItem` _listefruit))
  (`PrimitiveComponent.SetSimulatePhysics` (`/Game/bluprint/Cube/BP_Fruit.coco` _output) true)
  (`KismetArrayLibrary.Array_RemoveItem` _listefruit _output))

(fn `UserConstructionScript`)